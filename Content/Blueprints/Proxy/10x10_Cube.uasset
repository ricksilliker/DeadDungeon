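; Proxy 10x10 cube actor that gives itself a random color when play begins.
; The construction script creates a dynamic instance of the Proxy_RandColor material and stores it in Mat.
; BeginPlay sets that instance's "Base Color" parameter to random RGB values at full alpha, then applies it to the first material slot of the static mesh.
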(event EventBeginPlay
  (Rendering|Material|SetVectorParameterValue (Variables|Default|Getmat) "Base Color" (Utilities|Struct|MakeLinearColor (Math|Random|RandomFloatinRange 0.0 1.0) (Math|Random|RandomFloatinRange 0.0 1.0) (Math|Random|RandomFloatinRange 0.0 1.0) 1.0) :!class /Script/Engine.MaterialInstanceDynamic)
  (Rendering|Material|SetMaterial (Variables|Debug|GetStaticMeshComponent) 0 (Variables|Default|Getmat)))

(event Collision|EventActorBeginOverlap
  (params (OtherActor :type Actor%20Object%20Reference)))

(event EventTick
  (params (DeltaSeconds :type Float%20%28single-precision%29)))

(fn ConstructionScript
  (bind _returnvalue (Rendering|Material|CreateDynamicMaterialInstance "/Game/Mats/Proxy_RandColor.Proxy_RandColor" "ProxyCube" :!class /Script/Engine.KismetMaterialLibrary))
  (Variables|Default|Setmat _returnvalue))